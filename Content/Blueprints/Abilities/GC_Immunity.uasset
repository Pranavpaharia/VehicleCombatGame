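; GC_Immunity is a gameplay cue that shows an immunity shield as a sphere particle effect on a vehicle pawn.
; OnActive attaches the scaled emitter to the pawn's collision component and sets a timer by name for OnCloseShield on the spawned emitter, not on the cue.
; The cue's OnCloseShield is empty and OnRemove only calls the parent, so neither removes the effect.
; OnExecute only prints a debug string and calls the parent.
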(fn `OnActive`
  (params (MyTarget :type "Actor Object Reference") (Parameters :type "GameplayCueParameters Structure (by ref)"))
  (returns (ReturnValue :type Boolean))
  (bind _asvehicle_ue5pawn (cast `VehicleUE5Pawn` MyTarget))
  (bind _returnvalue (`GameplayStatics.SpawnEmitterAttached` "/Game/Stylized_Mobile_Effects/Particles/P_Abstract_Sphere.P_Abstract_Sphere" (`VehicleUE5Pawn.PawnCollisionComponent` _asvehicle_ue5pawn) "None" (0.0 0.0 0.0) (struct) (2.0 2.0 2.0)))
  (`KismetSystemLibrary.K2_SetTimer` _returnvalue "OnCloseShield" 4.0)
  (`KismetSystemLibrary.PrintString` MyTarget "IN GC_Immunity On Active ")
  (return (`parent.OnActive` MyTarget Parameters)))

(fn `OnCloseShield`)

(fn `OnExecute`
  (params (MyTarget :type "Actor Object Reference") (Parameters :type "GameplayCueParameters Structure (by ref)"))
  (returns (ReturnValue :type Boolean))
  (`KismetSystemLibrary.PrintString` MyTarget "GC_Immunity On Execute")
  (return (`parent.OnExecute` MyTarget Parameters)))

(fn `OnRemove`
  (params (MyTarget :type "Actor Object Reference") (Parameters :type "GameplayCueParameters Structure (by ref)"))
  (returns (ReturnValue :type Boolean))
  (return (`parent.OnRemove` MyTarget Parameters)))