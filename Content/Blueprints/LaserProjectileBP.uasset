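; Laser projectile that damages vehicle pawns through the Gameplay Ability System.
; On a swept overlap with a vehicle other than its instigator, the server adds the sweep hit result to the damage effect spec's context and applies it to that vehicle.
; The projectile then destroys itself, on both authority and remote.
; Disconnected leftovers include debug prints, a range-based lifespan and a line-trace alternative for finding the hit.
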(event `self.ReceiveBeginPlay`)

(event `self.ProjectileCollisionComponent.OnComponentBeginOverlap`
  (params (OverlappedComponent :type "PrimitiveComponent Object Reference") (OtherActor :type "Actor Object Reference") (OtherComp :type "PrimitiveComponent Object Reference") (OtherBodyIndex :type Integer) (bFromSweep :type Boolean) (SweepResult :type "HitResult Structure (by ref)"))
  (bind _returnvalue (`self.GetDamageEffectSpecHandle`))
  (if (!= OtherActor (`self.GetInstigator`))
    (`|ExecutionSequence`
      (:`then_1`
        (if bFromSweep
          (bind _asvehicle_ue5pawn (cast `VehicleUE5Pawn` (`.HitActor` (`GameplayStatics.BreakHitResult` SweepResult))))
          (`/Engine/EditorBlueprintResources/ActorMacros.Switch Has Authority`
            (:`Authority`
              (bind _output_get (set `self.ProjectileHitResult` SweepResult))
              (bind _returnvalue_2 (`AbilitySystemBlueprintLibrary.GetEffectContext` _returnvalue))
              (`AbilitySystemBlueprintLibrary.EffectContextAddHitResult` _returnvalue_2 _output_get)
              (`AbilitySystemComponent.BP_ApplyGameplayEffectSpecToSelf` (`AbilitySystemBlueprintLibrary.GetAbilitySystemComponent` _asvehicle_ue5pawn) _returnvalue)
              (`self.K2_DestroyActor`))
            (:`Remote`
              (`self.K2_DestroyActor`))))))))

(fn `UserConstructionScript`)