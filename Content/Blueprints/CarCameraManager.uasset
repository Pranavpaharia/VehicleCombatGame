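; CarCameraManager is a player camera manager that drives the view from the controlled vehicle's camera component.
; BlueprintUpdateCamera copies that camera's location, pitch, yaw and FOV but forces roll to zero, keeping the horizon level.
; GetPawnRef finds the vehicle through the camera target's owning VehiclePlayerControllerBP and caches both references, reporting invalid when the controller cast fails.
; OnRep_Car only prints the replicated car's name, and the EventGraph holds just unconnected network debug nodes.
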(event `self.ReceiveBeginPlay`)

(event `self.ReceiveTick`
  (params (DeltaSeconds :type "Float (single-precision)")))

(fn `BlueprintUpdateCamera`
  (params (CameraTarget :type "Actor Object Reference"))
  (returns (NewCameraLocation :type "Vector Structure") (NewCameraRotation :type "Rotator Structure") (NewCameraFOV :type "Float (single-precision)") (ReturnValue :type Boolean))
  (bind (_carpawn _valid) (`self.GetPawnRef` CameraTarget))
  (if _valid
    (bind _camera (`VehicleUE5Pawn.Camera` _carpawn))
    (bind (_returnvalue_roll _returnvalue_pitch _returnvalue_yaw) (`KismetMathLibrary.BreakRotator` (`SceneComponent.K2_GetComponentRotation` _camera)))
    (return (`SceneComponent.K2_GetComponentLocation` _camera) (`KismetMathLibrary.MakeRotator` 0.0 _returnvalue_pitch _returnvalue_yaw) (`CameraComponent.FieldOfView` _camera) _valid)
    (else
      (return (0.0 0.0 0.0) (struct) 0.0 false))))

(fn `GetPawnRef`
  (params (CameraRef :type "Actor Object Reference"))
  (returns (CarPawn :type "/Game/Blueprints/VehicleUE5PawnBP Object Reference") (Valid :type Boolean))
  (if (and (`KismetSystemLibrary.IsValid` (`self.Vehicle UE5Pawn BP`)) (`KismetSystemLibrary.IsValid` (`self.Vehicle Player ControllerBP`)))
    (return (`self.Vehicle UE5Pawn BP`) true)
    (else
      (bind _asvehicle_player_controller_bp (cast `/Game/Blueprints/VehiclePlayerControllerBP` (`self.GetOwner` CameraRef))
        (:`then`
          (bind _output_get (set `self.Vehicle Player ControllerBP` _asvehicle_player_controller_bp))
          (bind _asvehicle_ue5pawn_bp (cast `/Game/Blueprints/VehicleUE5PawnBP` (`Controller.K2_GetPawn` _output_get)))
          (bind _output_get_2 (set `self.Vehicle UE5Pawn BP` _asvehicle_ue5pawn_bp))
          (return _output_get_2 true))
        (:`CastFailed`
          (return null false))))))

(fn `OnRep_Car`
  (`KismetSystemLibrary.PrintString` (`KismetStringLibrary.Concat_StrStr` "Car Replicated Name: " (`KismetSystemLibrary.GetObjectName` (`self.Car`)))))

(fn `UserConstructionScript`)