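; Player controller for a vehicle game that sets up the welcome UI on BeginPlay according to network authority.
; Authority gets the offline welcome widget and background music, while remote clients get the online welcome widget.
; Player state and session ID events push the session string into the online widget.
; Touch input records position and a camera-move flag, but the camera rotation code is disconnected.
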(event `self.PlayUIClickSound`
  (`GameplayStatics.PlaySound2D` "/Game/Sounds/Sound_UIBasicClick.Sound_UIBasicClick" 1.0 1.0 0.0 null null))

(event `self.ReceiveActorOnInputTouchBegin`
  (params (FingerIndex :type "ETouchIndex Enum" :default "Touch1"))
  (switch `ETouchIndex` FingerIndex))

(event `self.ReceiveBeginPlay`
  (add `self.OnNewPlayerStateReceived` (delegate `PlayerStateReceived`))
  (set `self.bEnableTouchEvents` true)
  (`/Engine/EditorBlueprintResources/ActorMacros.Switch Has Authority`
    (:`Authority`
      (bind _returnvalue (`|CreateWidget` "/Game/Blueprints/Widgets/WB_WelcomeOfflineClient.WB_WelcomeOfflineClient_C"))
      (`UserWidget.AddToViewport` _returnvalue 0)
      (bind _output_get (set `self.Offline WidgetBox` _returnvalue))
      (`GameplayStatics.PlaySound2D` "/Game/Sounds/BackgroundMusic.BackgroundMusic" 1.0 1.0 0.0 null null)
      (`Widget.SetFocus` _output_get))
    (:`Remote`
      (bind _returnvalue_2 (`|CreateWidget` "/Game/Blueprints/Widgets/WB_OnlineClientWelcome.WB_OnlineClientWelcome_C"))
      (bind _output_get_2 (set `self.Online WidgetBox` _returnvalue_2))
      (`UserWidget.AddToViewport` _output_get_2 0))))

(event `PlayerStateReceived` :!signature `self.OnNewPlayerStateReceived`
  (params (NewPlayerState :type "VehiclePlayerState Object Reference"))
  (set `/Game/Blueprints/Widgets/WB_OnlineClientWelcome.SessionText` (`VehiclePlayerState.sessionStringID` NewPlayerState) (`self.Online WidgetBox`))
  (set `self.New Player State` NewPlayerState))

(event `self.ReceiveTick`
  (params (DeltaSeconds :type "Float (single-precision)"))
  (`/Engine/EditorBlueprintResources/StandardMacros.IsValid` (`self.New Player State`)))

(event `Key|Touch1`
  (params (Key :type "Key Structure"))
  (bind (_locationx _locationy _biscurrentlypressed) (`self.GetInputTouchState` "Touch1"))
  (:`Pressed`
    (set `self.bCameraMove` true)
    (set `self.CurrentPos` (`KismetMathLibrary.MakeVector2D` _locationx _locationy)))
  (:`Released`
    (set `self.bCameraMove` false)))

(event `SessionID Updated`
  (params (sessionstringID :type String))
  (bind _online_widgetbox (`self.Online WidgetBox`))
  (`/Engine/EditorBlueprintResources/StandardMacros.IsValid` _online_widgetbox
    (:`Is Valid`
      (set `/Game/Blueprints/Widgets/WB_OnlineClientWelcome.SessionText` sessionstringID _online_widgetbox))))

(fn `UserConstructionScript`)