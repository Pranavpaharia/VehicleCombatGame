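; Gameplay Cue notify actor that displays a sphere particle effect while an immunity cue is active on a vehicle pawn.
; OnActive casts the target to VehicleUE5Pawn, then sets the abstract sphere template on its own ParticleSystem component and activates it.
; OnRemove deactivates that component, and both handlers print debug strings.
; An alternative spawn-attached shield emitter is left disconnected and never runs.
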(fn `OnActive`
  (params (MyTarget :type "Actor Object Reference") (Parameters :type "GameplayCueParameters Structure (by ref)"))
  (returns (ReturnValue :type Boolean))
  (`KismetSystemLibrary.PrintString` MyTarget "IN GC_Immunity On Active ")
  (bind _asvehicle_ue5pawn (cast `VehicleUE5Pawn` MyTarget))
  (`ParticleSystemComponent.SetTemplate` (`self.ParticleSystem`) "/Game/Stylized_Mobile_Effects/Particles/P_Abstract_Sphere.P_Abstract_Sphere")
  (`ActorComponent.Activate` (`self.ParticleSystem`) true)
  (return true))

(fn `OnRemove`
  (params (MyTarget :type "Actor Object Reference") (Parameters :type "GameplayCueParameters Structure (by ref)"))
  (returns (ReturnValue :type Boolean))
  (`ActorComponent.Deactivate` (`self.ParticleSystem`))
  (`KismetSystemLibrary.PrintString` MyTarget "IN GC_Immunity Cue Deactivated!")
  (return true))

(fn `UserConstructionScript`)