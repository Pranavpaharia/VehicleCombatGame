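; Gameplay cue for a laser hit that plays impact feedback when executed.
; OnExecute spawns an enlarged impact emitter and a rocket-hit sound at the effect context's hit location, then calls the parent implementation.
; Disconnected leftover logic would play a fire sound for the instigator or a slowed explosion and death sound for killed vehicles, alongside an unused debug print.
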(fn `OnExecute`
  (params (MyTarget :type "Actor Object Reference") (Parameters :type "GameplayCueParameters Structure (by ref)"))
  (returns (ReturnValue :type Boolean))
  (bind (_bblockinghit _binitialoverlap _time _distance _location _impactpoint _normal _impactnormal _physmat _hitactor) (`GameplayStatics.BreakHitResult` (`AbilitySystemBlueprintLibrary.EffectContextGetHitResult` (`.EffectContext` (`AbilitySystemBlueprintLibrary.BreakGameplayCueParameters` Parameters)))))
  (`GameplayStatics.SpawnEmitterAtLocation` MyTarget "/Game/Stylized_Mobile_Effects/Particles/P_Impact_2.P_Impact_2" _location (struct) (3.0 3.0 3.0))
  (`GameplayStatics.PlaySoundAtLocation` MyTarget "/Game/Sounds/Sound_PlayerHitRocket.Sound_PlayerHitRocket" _location (struct) 1.0 1.0 0.0 null null null null)
  (return (`parent.OnExecute` MyTarget Parameters)))